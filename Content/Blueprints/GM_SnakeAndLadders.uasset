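; Game mode for a single-pawn, UI-only Snakes and Ladders game on a grid of widget blocks.
; BeginPlay creates the game widget, fills its grid and places the pawn on the bottom row.
; Each delayed dice roll moves the pawn along a serpentine path, then applies any snake or ladder jump.
; Rolls overshooting the top row are ignored, landing on the top-left cell ends the game, and restarting reloads the level.
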(event Custom|HandleDiceRoll
  (CallFunction|HandleRollingWait true)
  (Utilities|FlowControl|Delay 0.5)
  (CallFunction|HandleRollingWait false)
  (CallFunction|PerformDiceRoll)
  (bind (_jumptoposition _isjumposition) (CallFunction|CheckIsJumpPosition (Variables|Default|GetPawnPosition)))
  (if _isjumposition
    (Variables|/Game/Blueprints/WBP_Game.WBP_Game_C|SetIsRollEnabled (Variables|Default|GetGameWidgetRef) false)
    (Utilities|FlowControl|Delay 0.5)
    (Variables|/Game/Blueprints/WBP_Game.WBP_Game_C|SetIsRollEnabled (Variables|Default|GetGameWidgetRef) true)
    (CallFunction|UpdatePawnPosition _jumptoposition)))

(event EventBeginPlay
  (CallFunction|GenerateGameScene)
  (CallFunction|GenerateBoardGrid)
  (CallFunction|UpdatePawnPosition (Utilities|Struct|MakeStruct_GridPosition (.Row (Utilities|Struct|BreakStruct_GridPosition (Variables|Default|GetBoardSize))) 0)))

(fn ConstructionScript)

(fn PerformDiceRoll
  (bind _output_get (Variables|Default|SetCurrentDiceRoll (Math|Random|RandomIntegerinRange 1 6)))
  (CallFunction|UpdateDiceRollValue _output_get false)
  (bind _nextposition (CallFunction|ComputePawnNextPosition))
  (if (not (< (.Row (Utilities|Struct|BreakStruct_GridPosition _nextposition)) 0))
    (if (and (== (.Row (Utilities|Struct|BreakStruct_GridPosition _nextposition)) 0) (== (.Column (Utilities|Struct|BreakStruct_GridPosition _nextposition)) 0))
      (CallFunction|UpdatePawnPosition)
      (CallFunction|HandleGameOver)
      (else
        (CallFunction|UpdatePawnPosition _nextposition)))))

(fn UpdateDiceRollValue
  (params (DiceRollValue :type Integer) (IsDiceRolling :type Boolean))
  (bind _gamewidgetref (Variables|Default|GetGameWidgetRef))
  (if IsDiceRolling
    (bind _rolldotsformatted (CallFunction|GenerateDiceDots 99))
    (Variables|/Game/Blueprints/WBP_Game.WBP_Game_C|SetDiceRollValue (Variables|Default|GetGameWidgetRef) _rolldotsformatted)
    (elif (== DiceRollValue 0)
      (bind _rolldotsformatted_2 (CallFunction|GenerateDiceDots))
      (Variables|/Game/Blueprints/WBP_Game.WBP_Game_C|SetDiceRollValue _gamewidgetref _rolldotsformatted_2)
      (else
        (bind _rolldotsformatted_3 (CallFunction|GenerateDiceDots DiceRollValue))
        (Variables|/Game/Blueprints/WBP_Game.WBP_Game_C|SetDiceRollValue _gamewidgetref _rolldotsformatted_3)))))

(fn GenerateBoardGrid
  (Utilities|IsValid (Variables|Default|GetGameWidgetRef)
    (:Is%20Valid
      (for _index (range 0 9)
        (for _index_2 (range 0 9)
          (bind _returnvalue (UserInterface|CreateWidget "/Game/Blueprints/WBP_GridBlock.WBP_GridBlock_C" (Game|GetPlayerController 0)))
          (bind _returnvalue_2 (Class|UniformGridPanel|AddChildtoUniformGrid (Variables|/Game/Blueprints/WBP_Game.WBP_Game_C|GetBoardGridPanel (Variables|Default|GetGameWidgetRef)) _returnvalue _index _index_2))
          (Layout|GridSlot|SetHorizontalAlignment _returnvalue_2 "HAlign_Center")
          (Layout|GridSlot|SetVerticalAlignment _returnvalue_2 "VAlign_Center")
          (Utilities|Array|Add (Variables|Default|GetGridSlotsRef) (Utilities|Struct|MakeStruct_GridSlot _returnvalue (Utilities|Struct|MakeStruct_GridPosition _index _index_2))))))))

(fn GenerateGameScene
  (bind _returnvalue (UserInterface|CreateWidget "/Game/Blueprints/WBP_Game.WBP_Game_C" (Game|GetPlayerController 0)))
  (bind _output_get (Variables|Default|SetGameWidgetRef _returnvalue))
  (UserInterface|Viewport|AddtoViewport _output_get 0)
  (Input|SetInputModeUIOnly (Game|GetPlayerController 0) (Variables|Default|GetGameWidgetRef) "DoNotLock" false)
  (Variables|/Script/Engine.PlayerController|SetbShowMouseCursor (Game|GetPlayerController 0) true))

(fn UpdatePawnPosition
  (params (NewPawnPosition :type Struct%20Grid%20Position%20Structure))
  (Utilities|FlowControl|Sequence
    (:then_0
      (bind _slotref (CallFunction|FindGridSlotbyPosition (Variables|Default|GetPawnPosition)))
      (Variables|/Game/Blueprints/WBP_GridBlock.WBP_GridBlock_C|SetIsPawnVisible _slotref false))
    (:then_1
      (Variables|Default|SetPawnPosition NewPawnPosition)
      (bind _slotref_2 (CallFunction|FindGridSlotbyPosition NewPawnPosition))
      (Variables|/Game/Blueprints/WBP_GridBlock.WBP_GridBlock_C|SetIsPawnVisible _slotref_2 true))))

(fn FindGridSlotbyPosition
  (params (GridPosition :type Struct%20Grid%20Position%20Structure))
  (bind (_row _column) (Utilities|Struct|BreakStruct_GridPosition GridPosition))
  (for _array_element (Variables|Default|GetGridSlotsRef)
    (if (and (== (.row (.Position (Utilities|Struct|BreakStruct_GridSlot _array_element))) _row) (== (.column (.Position (Utilities|Struct|BreakStruct_GridSlot _array_element))) _column))
      (return (.SlotRef (Utilities|Struct|BreakStruct_GridSlot _array_element))))))

(fn ComputePawnNextPosition
  (bind _pawnposition (Variables|Default|GetPawnPosition))
  (bind _pawnposition_2 (Variables|Default|GetPawnPosition))
  (bind _pawnposition_3 (Variables|Default|GetPawnPosition))
  (bind _pawnposition_4 (Variables|Default|GetPawnPosition))
  (bind _boardsize (Variables|Default|GetBoardSize))
  (bind (_row _column) (Utilities|Struct|BreakStruct_GridPosition _pawnposition))
  (bind (_row_2 _column_2) (Utilities|Struct|BreakStruct_GridPosition _pawnposition_4))
  (bind _column_3 (Utilities|Struct|BreakStruct_GridPosition _boardsize))
  (bind (_row_3 _column_4) (Utilities|Struct|BreakStruct_GridPosition _pawnposition_2))
  (bind (_row_4 _column_5) (Utilities|Struct|BreakStruct_GridPosition _pawnposition_3))
  (if (== (Math|Integer|%(Integer) (+ (.Row (Utilities|Struct|BreakStruct_GridPosition (Variables|Default|GetPawnPosition))) 1) 2) 0)
    (if (<= (+ (.Column (Utilities|Struct|BreakStruct_GridPosition (Variables|Default|GetPawnPosition))) (Variables|Default|GetCurrentDiceRoll)) (.Column (Utilities|Struct|BreakStruct_GridPosition (Variables|Default|GetBoardSize))))
      (return (Utilities|Struct|MakeStruct_GridPosition _row_3 (+ _column_4 (Variables|Default|GetCurrentDiceRoll))))
      (else
        (return (Utilities|Struct|MakeStruct_GridPosition (- _row 1) (- (+ _column_3 1) (- (+ _column (Variables|Default|GetCurrentDiceRoll)) _column_3))))))
    (elif (>= (- (.Column (Utilities|Struct|BreakStruct_GridPosition (Variables|Default|GetPawnPosition))) (Variables|Default|GetCurrentDiceRoll)) 0)
      (return (Utilities|Struct|MakeStruct_GridPosition _row_4 (- _column_5 (Variables|Default|GetCurrentDiceRoll))))
      (else
        (return (Utilities|Struct|MakeStruct_GridPosition (- _row_2 1) (- (* (- _column_2 (Variables|Default|GetCurrentDiceRoll)) -1) 1)))))))

(fn HandleGameOver
  (Variables|/Game/Blueprints/WBP_Game.WBP_Game_C|SetIsGameOver (Variables|Default|GetGameWidgetRef) true))

(fn RestartGame
  (bind _returnvalue (Game|GetCurrentLevelName true))
  (Game|OpenLevel(byName) (Utilities|String|StringToName _returnvalue)))

(fn CheckIsJumpPosition
  (params (CurrentPosition :type Struct%20Grid%20Position%20Structure))
  (bind (_row _column) (Utilities|Struct|BreakStruct_GridPosition CurrentPosition))
  (bind (_row_2 _column_2) (Utilities|Struct|BreakStruct_GridPosition CurrentPosition))
  (bind _array_element (Utilities|Array|ForEachLoopwithBreak (Variables|Default|GetSnakePositions))
    (:LoopBody
      (if (and (== (.row (.StartPosition (Utilities|Struct|BreakStruct_GridPosition2x _array_element))) _row_2) (== (.column (.StartPosition (Utilities|Struct|BreakStruct_GridPosition2x _array_element))) _column_2))
        (return (.EndPosition (Utilities|Struct|BreakStruct_GridPosition2x _array_element)) true)))
    (:Completed
      (bind _array_element_2 (Utilities|Array|ForEachLoopwithBreak (Variables|Default|GetLadderPositions))
        (:LoopBody
          (if (and (== (.row (.StartPosition (Utilities|Struct|BreakStruct_GridPosition2x _array_element_2))) _row) (== (.column (.StartPosition (Utilities|Struct|BreakStruct_GridPosition2x _array_element_2))) _column))
            (return (.EndPosition (Utilities|Struct|BreakStruct_GridPosition2x _array_element_2)) true)))
        (:Completed
          (return "" false))))))

(fn HandleRollingWait
  (params (IsRolling :type Boolean))
  (bind _gamewidgetref (Variables|Default|GetGameWidgetRef))
  (CallFunction|UpdateDiceRollValue 0 IsRolling)
  (if IsRolling
    (Variables|/Game/Blueprints/WBP_Game.WBP_Game_C|SetIsRollEnabled _gamewidgetref false)
    (else
      (Variables|/Game/Blueprints/WBP_Game.WBP_Game_C|SetIsRollEnabled _gamewidgetref true))))

(fn GenerateDiceDots
  (params (DiceRollValue :type Integer))
  (switch int DiceRollValue
    (:Default
      (return (Utilities|Text|FormatText "Wait")))
    (:0
      (return (Utilities|Text|FormatText "Roll!")))
    (:1
      (return (Utilities|Text|FormatText "*")))
    (:2
      (return (Utilities|Text|FormatText "*  *")))
    (:3
      (return (Utilities|Text|FormatText "* * *")))
    (:4
      (return (Utilities|Text|FormatText "*   * 
*   *")))
    (:5
      (return (Utilities|Text|FormatText "* * * 
 *  *")))
    (:6
      (return (Utilities|Text|FormatText "* * * 
* * *")))))